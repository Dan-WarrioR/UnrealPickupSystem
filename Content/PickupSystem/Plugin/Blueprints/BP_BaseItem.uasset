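; Base pickup item actor that shows a mesh from its item data and can be collected on overlap.
; When animation is enabled, Tick spins the mesh and bobs the actor around its start location with a cosine-based height offset.
; With auto pickup on, overlapping actors implementing BPI_PickupReceiver trigger CallOnPicked, then receive the item data, and the item destroys itself if they accept.
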(event `self.ReceiveBeginPlay`
  (set `self.StartLocation` (`self.K2_GetActorLocation`)))

(event `self.ReceiveTick`
  (params (DeltaSeconds :type "Float (single-precision)"))
  (`self.ProceedAnimation` DeltaSeconds))

(event `self.PickupCollider.OnComponentBeginOverlap`
  (params (OverlappedComponent :type "PrimitiveComponent Object Reference") (OtherActor :type "Actor Object Reference") (OtherComp :type "PrimitiveComponent Object Reference") (OtherBodyIndex :type Integer) (bFromSweep :type Boolean) (SweepResult :type "HitResult Structure (by ref)"))
  (bind _itemdata (`self.ItemData`))
  (bind _asbpi_pickup_receiver (cast `/Game/PickupSystem/Plugin/Data/BPI_PickupReceiver` OtherActor))
  (if (`self.UseAutoPickup`)
    (`self.OnPicked` self _itemdata)
    (bind _success (`/Game/PickupSystem/Plugin/Data/BPI_PickupReceiver.OnPickupItem` _asbpi_pickup_receiver _itemdata self))
    (if _success
      (`self.K2_DestroyActor` self))))

(fn `ProceedAnimation`
  (params (DeltaSeconds :type "Float (double-precision)"))
  ; Rotation
  (if (`self.UseAnimation`)
    (`SceneComponent.K2_AddLocalRotation` (`self.ItemMesh`) (* (`self.RotationDelta`) DeltaSeconds) false false)
    ; Y Float
    (bind _output_get (set `self.RunningTime` (+ (`self.RunningTime`) DeltaSeconds)))
    (`self.K2_SetActorLocation` (+ (`self.StartLocation`) (`KismetMathLibrary.MakeVector` 0.0 0.0 (* (`KismetMathLibrary.Cos` (* _output_get (`self.FloatSpeed`))) (`self.FloatHeight`)))) false true)))

(fn `UserConstructionScript`
  (`StaticMeshComponent.SetStaticMesh` (`self.ItemMesh`) (`/Game/PickupSystem/Plugin/Data/BP_ItemInfo.ItemMesh` (`self.ItemData`))))