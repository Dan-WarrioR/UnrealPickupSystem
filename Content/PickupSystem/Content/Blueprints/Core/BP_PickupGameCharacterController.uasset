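; BP_PickupGameCharacterController is a controller that links player input to the BP_GameplayCharacter pawn in the pickup game.
; On BeginPlay it casts the first player's pawn, caches the reference, then runs the parent BeginPlay, which is skipped if the cast fails.
; Key events marked as a dev test call the pawn directly: E uses the item at index zero and R resets attributes.
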(event `self.ReceiveBeginPlay`
  (bind _asbp_gameplay_character (cast `/Game/PickupSystem/Content/Blueprints/BP_GameplayCharacter` (`GameplayStatics.GetPlayerPawn` 0)))
  (set `self.PlayerPawnRef` _asbp_gameplay_character)
  (`parent.ReceiveBeginPlay`))

(event `Key|E`
  (params (Key :type "Key Structure"))
  ; Dev test
  (:`Pressed`
    (`/Game/PickupSystem/Content/Blueprints/BP_GameplayCharacter.UseItem` (`self.PlayerPawnRef`) 0)))

(event `Key|R`
  (params (Key :type "Key Structure"))
  ; Dev test
  (:`Pressed`
    (`/Game/PickupSystem/Content/Blueprints/BP_GameplayCharacter.ResetAttributes` (`self.PlayerPawnRef`))))

(fn `UserConstructionScript`
  (`parent.UserConstructionScript`))