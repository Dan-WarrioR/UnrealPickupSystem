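; BP_GameplayCharacter is a character that holds a map-based item inventory and a map of numeric attributes.
; OnPickupItem adds or stacks items up to stack size, rejecting every pickup once the slot limit is reached, even stackable ones.
; UseItem takes a slot index, adds the item's values to matching attributes and decrements its stack.
; Inventory changes, attribute changes and ResetAttributes' zeroing are broadcast through BP_PickupGameState.
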(event `self.ReceiveBeginPlay`
  (bind _asbp_pickup_game_state (cast `/Game/PickupSystem/Content/Blueprints/Core/BP_PickupGameState` (`GameplayStatics.GetGameState`)))
  (set `self.GameStateRef` _asbp_pickup_game_state))

(fn `OnPickupItem`
  (params (ItemData :type "/Game/PickupSystem/Plugin/Data/BP_ItemInfo Object Reference (by ref)") (ItemActorRef :type "Actor Object Reference (by ref)"))
  (returns (Success :type Boolean))
  (bind _inventory (`self.Inventory`))
  (bind _value (`BlueprintMapLibrary.Map_Find` (`self.Inventory`) ItemData))
  (if (< (`BlueprintMapLibrary.Map_Length` (`self.Inventory`)) (`self.InventoryMaxAmount`))
    (if (`BlueprintMapLibrary.Map_Contains` (`self.Inventory`) ItemData)
      (if (== _value (`/Game/PickupSystem/Plugin/Data/BP_ItemInfo.StackSize` ItemData))
        (`KismetSystemLibrary.PrintText` "Full Stack for item" true true (struct :`R` 1.0 :`A` 1.0) 1.0)
        (return false)
        (else
          (bind _result (`/Engine/EditorBlueprintResources/StandardMacros.IncrementInt` _value)
            (:`  `
              (`BlueprintMapLibrary.Map_Add` _inventory ItemData _result)))))
      (else
        (`BlueprintMapLibrary.Map_Add` _inventory ItemData 1)))
    (`/Game/PickupSystem/Content/Blueprints/Core/BP_PickupGameState.OnInventoryUpdated` (`self.GameStateRef`) (`self.Inventory`))
    (return true)
    (else
      (`KismetSystemLibrary.PrintText` "Full Inventory" true true (struct :`R` 1.0 :`A` 1.0) 1.0)
      (return false))))

(fn `ResetAttributes`
  (bind _attributesmap (`self.AttributesMap`))
  (bind _keypin (`|MapForEach` _attributesmap)
    (:`then`
      (`BlueprintMapLibrary.Map_Add` (`self.AttributesMap`) _keypin))
    (:`CompletedPin`
      (`/Game/PickupSystem/Content/Blueprints/Core/BP_PickupGameState.OnCharacterAttributesChanged` (`self.GameStateRef`) _attributesmap))))

(fn `UseItem`
  (params (ItemSlotIndex :type Integer))
  (bind _attributesmap (`self.AttributesMap`))
  (bind _inventory (`self.Inventory`))
  (bind (_key _value) (`BlueprintMapLibrary.Map_GetKeyValueByIndex` (`self.Inventory`) ItemSlotIndex))
  (bind _returnvalue (`BlueprintMapLibrary.Map_Length` (`self.Inventory`)))
  (bind _attributes_attributes (break `/Game/PickupSystem/Plugin/Data/S_ItemAttributes` (`/Game/PickupSystem/Plugin/Data/BP_ItemInfo.Attributes` _key)))
  (if (and (> _returnvalue 0) (>= ItemSlotIndex 0) (< ItemSlotIndex _returnvalue))
    (bind (_keypin _valuepin) (`|MapForEach` _attributes_attributes)
      (:`then`
        (bind (_value_2 _returnvalue_2) (`BlueprintMapLibrary.Map_Find` _attributesmap _keypin))
        ; Attributes
        (if _returnvalue_2
          (`BlueprintMapLibrary.Map_Add` _attributesmap _keypin (+ _value_2 _valuepin))
          (`/Game/PickupSystem/Content/Blueprints/Core/BP_PickupGameState.OnCharacterAttributesChanged` (`self.GameStateRef`) (`self.AttributesMap`))))
      (:`CompletedPin`
        ; Item Slot Update
        (bind _result (`/Engine/EditorBlueprintResources/StandardMacros.DecrementInt` _value)
          (:`  `
            (if (<= _result 0)
              (`BlueprintMapLibrary.Map_Remove` _inventory _key)
              (else
                (`BlueprintMapLibrary.Map_Add` _inventory _key _result)))
            (`/Game/PickupSystem/Content/Blueprints/Core/BP_PickupGameState.OnInventoryUpdated` (`self.GameStateRef`) _inventory)))))
    (else
      (return))))

(fn `UserConstructionScript`
  (`parent.UserConstructionScript`))